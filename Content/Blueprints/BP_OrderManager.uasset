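; BP_OrderManager keeps the queue of customer orders and tracks which one is current.
; AddOrder stores each order as Ordered with its customer, notifies that customer, and marks the order Active if it is alone in the array.
; CompleteCurrentOrder marks the current entry Completed without removing it, then notifies the customer and advances CurrentIndex only if that customer is valid.
; Both functions broadcast OnOrderUpdated after successful changes.
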(fn `AddOrder`
  (params (NewOrder :type "/Game/Data/S_Orders Structure") (CustomerRef :type "/Game/Characters/Customer/BP_GenericCustomer Object Reference"))
  (bind _activeorders (`self.ActiveOrders`))
  (bind _structout (setmembers `/Game/Data/S_Orders` :`StructRef` NewOrder :`Status` (struct :`TagName` "Status.Ordered") :`CustomerRef` CustomerRef))
  (`KismetArrayLibrary.Array_Add` _activeorders _structout)
  (`/Game/Characters/Customer/BP_GenericCustomer.OnOrderTaken` (`.CustomerRef_26_9C89A326480EFA64BE07D2B2E3CF1417` (break `/Game/Data/S_Orders` _structout)))
  (if (== (`KismetArrayLibrary.Array_Length` _activeorders) 1)
    (bind _structout_2 (setmembers `/Game/Data/S_Orders` :`StructRef` (`|GetArrayItem` _activeorders) :`Status` (struct :`TagName` "Status.Active")))
    (`KismetArrayLibrary.Array_Set` _activeorders 0 _structout_2))
  (`self.OnOrderUpdated`))

(fn `CompleteCurrentOrder`
  (bind _activeorders (`self.ActiveOrders`))
  (bind _currentindex (`self.CurrentIndex`))
  (bind _returnvalue (`KismetArrayLibrary.Array_Length` _activeorders))
  (bind _output (`|GetArrayItem` _activeorders _currentindex))
  (bind (_orderid _ordertype _ordername _description _status _customerref) (break `/Game/Data/S_Orders` _output))
  (if (>= _currentindex _returnvalue)
    (return)
    (else
      (bind _structout (setmembers `/Game/Data/S_Orders` :`StructRef` _output :`Status` (struct :`TagName` "Status.Completed")))
      (`KismetArrayLibrary.Array_Set` _activeorders _currentindex _structout)
      (`/Engine/EditorBlueprintResources/StandardMacros.IsValid` _customerref
        (:`Is Valid`
          (`/Game/Characters/Customer/BP_GenericCustomer.OnOrderCompleted` _customerref)
          (bind _result (`/Engine/EditorBlueprintResources/StandardMacros.IncrementInt` _currentindex)
            (:`  `
              (if (< _result _returnvalue)
                (setmembers `/Game/Data/S_Orders` :`StructRef` _output :`Status` (struct :`TagName` "Status.Active"))
                (`KismetArrayLibrary.Array_Set` _activeorders _result))
              (`self.OnOrderUpdated`))))))))

(fn `UserConstructionScript`)