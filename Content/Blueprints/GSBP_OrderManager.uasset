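; Order manager that tracks a list of orders and their status.
; AddOrder appends each order as Ordered, promotes it to Active if it is the only entry, then calls OnOrderUpdated.
; CompleteCurrentOrder marks the entry at CurrentIndex as Completed and advances the index, without setting the next order Active.
; Completed orders stay in the ActiveOrders array.
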(fn `AddOrder`
  (params (NewOrder :type "/Game/Data/S_Orders Structure"))
  (bind _activeorders (`self.ActiveOrders`))
  (bind _structout (setmembers `/Game/Data/S_Orders` :`StructRef` NewOrder :`Status` (struct :`TagName` "Status.Ordered")))
  (`KismetArrayLibrary.Array_Add` _activeorders _structout)
  (if (== (`KismetArrayLibrary.Array_Length` _activeorders) 1)
    (bind _structout_2 (setmembers `/Game/Data/S_Orders` :`StructRef` (`|GetArrayItem` _activeorders) :`Status` (struct :`TagName` "Status.Active")))
    (`KismetArrayLibrary.Array_Set` _activeorders 0 _structout_2))
  (`self.OnOrderUpdated`))

(fn `CompleteCurrentOrder`
  (bind _activeorders (`self.ActiveOrders`))
  (bind _currentindex (`self.CurrentIndex`))
  (bind _returnvalue (`KismetArrayLibrary.Array_Length` _activeorders))
  (if (not (>= _currentindex _returnvalue))
    (bind _structout (setmembers `/Game/Data/S_Orders` :`StructRef` (`|GetArrayItem` _activeorders _currentindex) :`Status` (struct :`TagName` "Status.Completed") :!label _label))
    (`KismetArrayLibrary.Array_Set` _activeorders _currentindex _structout)
    (bind _result (`/Engine/EditorBlueprintResources/StandardMacros.IncrementInt` _currentindex)
      (:`  `
        (if (>= _result _returnvalue)
          (goto _label)
          (else
            _)))))
  (`self.OnOrderUpdated`))

(fn `UserConstructionScript`)