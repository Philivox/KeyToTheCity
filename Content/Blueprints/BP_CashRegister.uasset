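; BP_CashRegister is a register where the player takes orders from waiting customers.
; Customer and Worker overlap volumes track who is present, store the customer, and show a take-order widget when the player arrives while a customer waits.
; TakeOrder picks a random DT_Orders row if both are present.
; Its second sequence step, outside that check, passes the row and stored customer to the first BP_OrderManager found.
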(event `self.Customer.OnComponentBeginOverlap`
  (params (OverlappedComponent :type "PrimitiveComponent Object Reference") (OtherActor :type "Actor Object Reference") (OtherComp :type "PrimitiveComponent Object Reference") (OtherBodyIndex :type Integer) (bFromSweep :type Boolean) (SweepResult :type "HitResult Structure (by ref)"))
  ; Customer Overlapping
  (bind _asbp_generic_customer (cast `/Game/Characters/Customer/BP_GenericCustomer` OtherActor))
  (`/Engine/EditorBlueprintResources/StandardMacros.IsValid` _asbp_generic_customer
    (:`Is Valid`
      (set `self.CustomerRef` _asbp_generic_customer) ; Set the customer here to pass into TakeOrder function
      (set `self.IsCustomerWaiting?` true))))

(event `self.Customer.OnComponentEndOverlap`
  (params (OverlappedComponent :type "PrimitiveComponent Object Reference") (OtherActor :type "Actor Object Reference") (OtherComp :type "PrimitiveComponent Object Reference") (OtherBodyIndex :type Integer))
  ; Customer Overlapping
  (cast `/Game/Characters/Customer/BP_GenericCustomer` OtherActor)
  (set `self.IsCustomerWaiting?` false))

(event `self.Worker.OnComponentBeginOverlap`
  (params (OverlappedComponent :type "PrimitiveComponent Object Reference") (OtherActor :type "Actor Object Reference") (OtherComp :type "PrimitiveComponent Object Reference") (OtherBodyIndex :type Integer) (bFromSweep :type Boolean) (SweepResult :type "HitResult Structure (by ref)"))
  ; Player Overlapping
  (cast `/Game/Blueprints/BP_MainPlayer` OtherActor)
  (set `self.IsPlayerAtRegister` true)
  (if (`self.IsCustomerWaiting?`)
    (`SceneComponent.SetVisibility` (`self.W_TakeOrder`) true false)))

(event `self.Worker.OnComponentEndOverlap`
  (params (OverlappedComponent :type "PrimitiveComponent Object Reference") (OtherActor :type "Actor Object Reference") (OtherComp :type "PrimitiveComponent Object Reference") (OtherBodyIndex :type Integer))
  ; Player Overlapping
  (cast `/Game/Blueprints/BP_MainPlayer` OtherActor)
  (set `self.IsPlayerAtRegister` false)
  (`SceneComponent.SetVisibility` (`self.W_TakeOrder`) false false))

(fn `TakeOrder`
  (`|ExecutionSequence`
    (:`then_0`
      (if (and (`self.IsCustomerWaiting?`) (`self.IsPlayerAtRegister`))
        (bind _outrownames (`DataTableFunctionLibrary.GetDataTableRowNames` "/Game/Data/DT_Orders.DT_Orders"))
        (bind _returnvalue (`|GetDataTableRow` "/Game/Data/DT_Orders.DT_Orders" (`|GetArrayItem` _outrownames (`KismetMathLibrary.RandomIntegerInRange` 0 (- (`KismetArrayLibrary.Array_Length` _outrownames) 1)))))))
    (:`then_1`
      (bind _outactors (`GameplayStatics.GetAllActorsOfClass` "/Game/Blueprints/BP_OrderManager.BP_OrderManager_C"))
      (`/Game/Blueprints/BP_OrderManager.AddOrder` (`|GetArrayItem` _outactors) _returnvalue (`self.CustomerRef`)))))

(fn `UserConstructionScript`)