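; BP_KitchenZone is the kitchen station trigger that lets the player start typing when a kitchen order is active.
; On PrepTrigger overlap by BP_MainPlayer, it searches BP_OrderManager's ActiveOrders for an active Kitchen order and enables typing.
; Without a match in a non-empty list, a DoOnce briefly shows a wrong-zone widget.
; Leaving the trigger disables typing and resets the DoOnce.
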(event `self.PrepTrigger.OnComponentBeginOverlap`
  (params (OverlappedComponent :type "PrimitiveComponent Object Reference") (OtherActor :type "Actor Object Reference") (OtherComp :type "PrimitiveComponent Object Reference") (OtherBodyIndex :type Integer) (bFromSweep :type Boolean) (SweepResult :type "HitResult Structure (by ref)"))
  (bind _asbp_main_player (cast `/Game/Blueprints/BP_MainPlayer` OtherActor))
  (bind _returnvalue (`GameplayStatics.GetActorOfClass` "/Game/Blueprints/BP_OrderManager.BP_OrderManager_C"))
  (bind _activeorders (`/Game/Blueprints/BP_OrderManager.ActiveOrders` _returnvalue))
  ; This logic is crazy but it's just finding the first one that matches OrderType status and is Active
  (if (not (`KismetArrayLibrary.Array_IsEmpty` _activeorders))
    (for _array_element _activeorders
      (bind (_orderid _ordertype _ordername _description _status) (break `/Game/Data/S_Orders` _array_element))
      (if (and (== _ordertype (struct :`TagName` "OrderType.Kitchen")) (== _status (struct :`TagName` "Status.Active")))
        (bind _output_get (set `self.bFoundMatchingOrder` true))
        (break)))
    (if _output_get
      (`/Game/Blueprints/BP_MainPlayer.SetCanStartTyping` _asbp_main_player true)
      (set `self.bFoundMatchingOrder` false)
      (else
        (`/Engine/EditorBlueprintResources/StandardMacros.DoOnce` false :!label _label
          (:`Completed`
            (bind _returnvalue_2 (`|CreateWidget` "/Game/Widgets/WBP_WrongZoneMsg.WBP_WrongZoneMsg_C"))
            (`UserWidget.AddToViewport` _returnvalue_2 0)
            (`KismetSystemLibrary.Delay` 1.5)
            (`Widget.RemoveFromParent` _returnvalue_2)))))))

(event `self.PrepTrigger.OnComponentEndOverlap`
  (params (OverlappedComponent :type "PrimitiveComponent Object Reference") (OtherActor :type "Actor Object Reference") (OtherComp :type "PrimitiveComponent Object Reference") (OtherBodyIndex :type Integer))
  (bind _asbp_main_player (cast `/Game/Blueprints/BP_MainPlayer` OtherActor))
  (`/Game/Blueprints/BP_MainPlayer.SetCanStartTyping` _asbp_main_player false)
  (goto _label :!via `Reset`))

(fn `UserConstructionScript`)