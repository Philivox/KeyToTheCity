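; BP_CustomerSpawn runs a timed shop shift and spawns BP_GenericCustomer actors at random points inside its SpawnVolume.
; ShiftStart plays a sound, briefly shows a start widget, then starts the shift-length timer and a looping spawn timer whose random interval is rolled once per shift.
; ShiftEnd clears both timers, briefly shows an end widget with sound, then calls the shift-end dispatcher.
; A SpawnCustomer function duplicates the timer-driven spawn logic.
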(event `SpawnCust`
  (bind _spawnvolume (`self.SpawnVolume`))
  (`|SpawnActorFromClass` "/Game/Characters/Customer/BP_GenericCustomer.BP_GenericCustomer_C" (`KismetMathLibrary.Conv_VectorToTransform` (`KismetMathLibrary.RandomPointInBoundingBox` (`SceneComponent.K2_GetComponentLocation` _spawnvolume) (`BoxComponent.GetScaledBoxExtent` _spawnvolume))) "AdjustIfPossibleButDontSpawnIfColliding" "MultiplyWithRoot" null null))

(event `ShiftStart`
  (`GameplayStatics.PlaySound2D` "/Game/Imports/Sounds/shop-open.shop-open" 1.0 1.0 0.0 null null)
  (bind _returnvalue (`|CreateWidget` "/Game/Widgets/WBP_StartShift.WBP_StartShift_C" (`GameplayStatics.GetPlayerController` 0)))
  (`UserWidget.AddToViewport` _returnvalue 0)
  (`KismetSystemLibrary.Delay` 2.0)
  (`Widget.RemoveFromParent` _returnvalue)
  (bind _returnvalue_2 (`KismetSystemLibrary.K2_SetTimerDelegate` (delegate `ShiftEnd`) (`self.ShiftLength`)))
  (set `self.ShiftTimerHandle` _returnvalue_2)
  (bind _returnvalue_3 (`KismetSystemLibrary.K2_SetTimerDelegate` (delegate `SpawnCust`) (`KismetMathLibrary.Conv_IntToDouble` (`KismetMathLibrary.RandomIntegerInRange` 5 10)) true))
  (set `self.CustomerSpawnTimerHandle` _returnvalue_3))

(event `ShiftEnd`
  (`KismetSystemLibrary.K2_ClearAndInvalidateTimerHandle` (`self.CustomerSpawnTimerHandle`))
  (`KismetSystemLibrary.K2_ClearAndInvalidateTimerHandle` (`self.ShiftTimerHandle`))
  (bind _returnvalue (`|CreateWidget` "/Game/Widgets/WBP_EndShift.WBP_EndShift_C" (`GameplayStatics.GetPlayerController` 0)))
  (`UserWidget.AddToViewport` _returnvalue 0)
  (`KismetSystemLibrary.Delay` 2.0)
  (`GameplayStatics.PlaySound2D` "/Game/Imports/Sounds/shop-open.shop-open" 1.0 1.0 0.0 null null)
  (`Widget.RemoveFromParent` _returnvalue)
  (`self.ShiftEndDispatcher`))

(fn `SpawnCustomer`
  (bind _spawnvolume (`self.SpawnVolume`))
  (`|SpawnActorFromClass` "/Game/Characters/Customer/BP_GenericCustomer.BP_GenericCustomer_C" (`KismetMathLibrary.Conv_VectorToTransform` (`KismetMathLibrary.RandomPointInBoundingBox` (`SceneComponent.K2_GetComponentLocation` _spawnvolume) (`BoxComponent.GetScaledBoxExtent` _spawnvolume))) "AdjustIfPossibleButDontSpawnIfColliding" "MultiplyWithRoot" null null))

(fn `UserConstructionScript`)